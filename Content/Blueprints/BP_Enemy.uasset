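; Enemy Blueprint that spawns with a random look, takes damage and dies as a ragdoll.
; BeginPlay assigns a skeletal mesh picked at random from the RandomSkelethal collection.
; AnyDamage subtracts from clamped health and calls Death when it reaches zero.
; Death enables collision and physics simulation on the mesh, then destroys the actor after a delay.
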(event `self.ReceiveBeginPlay`
  ;[1 1 1] Random Mesh
  (`SkeletalMeshComponent.SetSkeletalMeshAsset` (`self.Mesh`) (`KismetArrayLibrary.Array_Random` (`self.RandomSkelethal`))))

(event `self.ReceiveAnyDamage`
  (params (Damage :type "Float (single-precision)") (DamageType :type "DamageType Object Reference") (InstigatedBy :type "Controller Object Reference") (DamageCauser :type "Actor Object Reference"))
  ;[1 1 1] Damage
  (set `self.Ennemy Health` (`KismetMathLibrary.FClamp` (- (`self.Ennemy Health`) Damage) 0.0 100.0))
  (if (<= (`self.Ennemy Health`) 0.0)
    (`self.Death`)))

(event `Death`
  (bind _mesh (`self.Mesh`))
  ;[1 1 1] Ragdoll and death
  (`PrimitiveComponent.SetCollisionEnabled` _mesh "QueryAndPhysics")
  (`PrimitiveComponent.SetSimulatePhysics` _mesh true)
  (`SkeletalMeshComponent.SetPhysicsBlendWeight` _mesh 1.0)
  (`KismetSystemLibrary.Delay` 10.0)
  (`self.K2_DestroyActor`))

(fn `UserConstructionScript`)